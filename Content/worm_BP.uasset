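; worm_BP is a side-scroller hazard that patrols back and forth and marks the player character dead on hit.
; WormTimeline starts at BeginPlay and drives a lerp of its relative location between StartPoint and EndPoint, with MovementRate as a speed divisor.
; When the timeline finishes, the worm waits WaitTime, turns around and plays the timeline in the opposite direction.
; A hit on RenderComponent sets PlayerDead on the 2DSideScrollerCharacter.
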(event `self.ReceiveBeginPlay`
  ;[1 1 1] Makes the fly go back and forth
  (bind (_direction _movementtime) (`Timeline|WormTimeline` :`NewTime` (/ (`TimelineComponent.GetPlayRate` (`self.WormTimeline`)) (`self.MovementRate`)) :!label _label)
    (:`Update`
      (`self.K2_SetActorRelativeLocation` (`KismetMathLibrary.VLerp` (`self.StartPoint`) (`self.EndPoint`) _movementtime)))
    (:`Finished`
      (`KismetSystemLibrary.Delay` (`self.WaitTime`))
      (switch `ETimelineDirection` (select `ETimelineDirection` _direction :`Forward` "Backward" :`Backward` "Forward" :!type "ETimelineDirection Enum")
        (:`Forward`
          (`self.SetActorRotation` (struct))
          (goto _label :!via `PlayFromStart`))
        (:`Backward`
          (`self.SetActorRotation` (struct :`Yaw` 180.0))
          (goto _label :!via `ReverseFromEnd`))))))

(event `self.RenderComponent.OnComponentHit`
  (params (OtherActor :type "Actor Object Reference") (OtherComp :type "PrimitiveComponent Object Reference") (NormalImpulse :type "Vector Structure") (Hit :type "HitResult Structure (by ref)"))
  (bind _as2dside_scroller_character (cast `/Game/2DSideScrollerBP/Blueprints/2DSideScrollerCharacter` OtherActor))
  (set `/Game/2DSideScrollerBP/Blueprints/2DSideScrollerCharacter.PlayerDead` true _as2dside_scroller_character))

(event `self.ReceiveActorBeginOverlap`
  (params (OtherActor :type "Actor Object Reference")))

(event `self.ReceiveTick`
  (params (DeltaSeconds :type "Float (single-precision)")))

(fn `UserConstructionScript`)